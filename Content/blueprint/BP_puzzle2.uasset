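; Sliding number puzzle that spawns a grid of numbered TEST tiles at BeginPlay, hiding the zero tile as the empty slot.
; Clicking a tile runs a sphere overlap around it to check whether the hidden tile is a neighbour.
; If so, two chained timelines lerp the tile into the gap, then the hidden tile into the vacated spot, with click events disabled meanwhile.
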(event Custom|click
  (params (TouchedActor :type Actor%20Object%20Reference) (ButtonPressed :type Key%20Structure :default "None"))
  (bind _astest (Utilities|Casting|CastToTEST TouchedActor))
  (bind _output_get (Variables|Default|SetTouched%20Actor _astest))
  (EventDispatchers|BindEventtoOnClicked _output_get (delegate Custom|click))
  (bind _neighbours (CallFunction|Getneighbours))
  (CallFunction|Getmoveto _neighbours)
  (Utilities|IsValid (Variables|Default|Getmovetotarget)
    (:Is%20Valid
      (CallFunction|Moveto))))

(event Custom|move%20to
  (bind _touched_actor (Variables|Default|GetTouched%20Actor))
  (bind _returnvalue (Transformation|GetActorLocation _touched_actor))
  (Variables|/Script/Engine.PlayerController|SetbEnableClickEvents (Game|GetPlayerController 0) false)
  (Variables|Default|Setmovetostart _returnvalue)
  (Variables|Default|Setactorpos _returnvalue)
  (bind _newtrack_0 (Timeline|Timeline PlayFromStart)
    (:Update
      (Transformation|SetActorLocation (Variables|Default|GetTouched%20Actor) (Math|Vector|Lerp(Vector) (Variables|Default|Getmovetostart) (Transformation|GetActorLocation (Variables|Default|Getmovetotarget)) _newtrack_0) false false))
    (:Finished
      (bind _newtrack_0_2 (Timeline|Timeline_0 PlayFromStart)
        (:Update
          (Transformation|SetActorLocation (Variables|Default|Getbox0) (Math|Vector|Lerp(Vector) (Transformation|GetActorLocation (Variables|Default|Getbox0)) (Variables|Default|Getactorpos) _newtrack_0_2) false false))
        (:Finished
          (Variables|/Script/Engine.PlayerController|SetbEnableClickEvents (Game|GetPlayerController 0) true))))))

(event EventBeginPlay
  (bind _returnvalue (Transformation|GetActorLocation))
  (for _index (range 0 (Variables|Default|Getgridsize))
    (bind _returnvalue_2 (Game|SpawnActorfromClass "/Game/blueprint/TEST.TEST_C" (Math|Transform|MakeTransform (Math|Vector|MakeVector (+ (Math|Conversions|ToFloat(Integer) (* (Math|Integer|%(Integer) _index (Variables|Default|Getsquaredivide)) (Variables|Default|GetSpacing))) (.x _returnvalue)) (.y _returnvalue) (+ (Math|Conversions|ToFloat(Integer) (* (/ _index (Variables|Default|Getsquaredivide)) (* (Variables|Default|GetSpacing) -1))) (.z _returnvalue))) "0, 0, 0" "1.000000,1.000000,1.000000") "Undefined" "MultiplyWithRoot" 0 0))
    (bind _returnvalue_3 (Utilities|Array|Add (Variables|Default|Getpuzzle) _returnvalue_2))
    (Rendering|Components|TextRender|SetText (Variables|/Game/blueprint/TEST.TEST_C|GetTextRender _returnvalue_2) (Utilities|Text|ToText(Integer) (Utilities|Array|Get(acopy) (Variables|Default|Getnumber) _index)))
    (if (Utilities|Enum|Equal(Enum) (Utilities|Text|ToText(Integer) (Utilities|Array|Get(acopy) (Variables|Default|Getnumber) _index)) (Utilities|Text|MakeLiteralText "0"))
      (Rendering|SetActorHiddenInGame (Utilities|Array|Get(acopy) (Variables|Default|GetPuzzle) _returnvalue_3) true)
      (Variables|Default|Setbox0 (Utilities|Array|Get(acopy) (Variables|Default|GetPuzzle) _returnvalue_3))))
  (for _array_element (Variables|Default|GetPuzzle)
    (EventDispatchers|BindEventtoOnClicked _array_element (delegate Custom|click))))

(event Collision|EventActorBeginOverlap
  (params (OtherActor :type Actor%20Object%20Reference)))

(event EventTick
  (params (DeltaSeconds :type Float%20%28single-precision%29)))

(fn ConstructionScript)

(fn Getneighbours
  (bind _outactors (Collision|SphereOverlapActors (Transformation|GetActorLocation (Variables|Default|GetTouched%20Actor)) (Variables|Default|Getmeshsize) (Utilities|Array|MakeArray "ObjectTypeQuery1" "ObjectTypeQuery2") "/Script/Engine.Actor"))
  (return _outactors))

(fn Getmoveto
  (params (neighbourslist :type Array%20of%20Actor%20Object%20References))
  (Variables|Default|Setmovetotarget 0)
  (for _array_element neighbourslist
    (if (== _array_element (Variables|Default|Getbox0))
      (Variables|Default|Setmovetotarget _array_element)))
  (return))